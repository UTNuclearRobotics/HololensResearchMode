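; HoloLens sensor publisher that streams one camera or depth scanner, chosen by SensorType, as mono8 image messages.
; BeginPlay builds the topic name from the enum, creates the sensor and starts capture.
; Once its texture exists, it listens for PublishMonoCamera events, which set a timer that publishes frames, or a stop message when publishing is off.
; Both depth scanner types read short-throw data and reuse the VLC publish call.
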(event `self.ReceiveBeginPlay`
  ;[1 1 1] Event Begin Play
  (`self.ConfigSensorTopicName`)
  (`self.CreateSensorObject`))

(event `ConfigSensorTopicName`
  (bind _returnvalue (`KismetStringLibrary.Replace` (`|GetEnumeratorNameAsString` (`self.Sensor Type`)) " "))
  ;[1 1 1] Topic Name Configuration
  (switch `EHololensSensorType` (`self.Sensor Type`)
    (:`LEFT_FRONT`
      (set `self.PostfixTopicName` "/image/raw" :!label _label))
    (:`LEFT_LEFT`
      (goto _label))
    (:`RIGHT_FRONT`
      (goto _label))
    (:`RIGHT_RIGHT`
      (goto _label))
    (:`DEPTH_AHAT`
      (set `self.PostfixTopicName` "/image/depth" :!label _label_2))
    (:`DEPTH_LONG_THROW`
      (goto _label_2)))
  (bind _output_get (set `self.PrefixTopicName` _returnvalue))
  (bind _output_get_2 (set `self.ImageTopicName` (`KismetStringLibrary.Concat_StrStr` _output_get (`self.PostfixTopicName`))))
  (`KismetSystemLibrary.PrintString` (`KismetStringLibrary.Concat_StrStr` _returnvalue " sensor image topic: " _output_get_2)))

(event `CreateSensorObject`
  (bind _sensor_type (`self.Sensor Type`))
  ;[1 1 1] Setup Sensor Objects
  (bind _returnvalue (`HololensResearchModeFunctionLibrary.CreateSensor` _sensor_type self))
  (switch `EHololensSensorType` _sensor_type
    (:`LEFT_FRONT`
      (bind _ashololens_vlccam (cast `HololensVLCCam` _returnvalue :!label _label_3))
      (bind _output_get (set `self.As Hololens VLCCam` _ashololens_vlccam))
      (add `HololensCameraSensor.OnVideoTextureCreated` _output_get (delegate `OnVLCTextureCreationSuccess`))
      (`HololensSensor.StartCapturing` (`self.As Hololens VLCCam`)))
    (:`LEFT_LEFT`
      (goto _label_3))
    (:`RIGHT_FRONT`
      (goto _label_3))
    (:`RIGHT_RIGHT`
      (goto _label_3))
    (:`DEPTH_AHAT`
      (bind _ashololens_depth_cam (cast `HololensDepthCam` _returnvalue :!label _label_4))
      (bind _output_get_2 (set `self.As Hololens Depth Cam` _ashololens_depth_cam))
      (add `HololensCameraSensor.OnVideoTextureCreated` _output_get_2 (delegate `OnDepthTextureCreationSuccess`))
      (`HololensSensor.StartCapturing` (`self.As Hololens Depth Cam`)))
    (:`DEPTH_LONG_THROW`
      (goto _label_4))))

(event `OnVLCTextureCreationSuccess`
  (params (InSensor :type "HololensCameraSensor Object Reference"))
  ;[1 1 1] Setup Sensor Objects
  (`self.SetupPublishVLCImageMessageListener` (stale `CreateSensorObject` _output_get)))

(event `OnDepthTextureCreationSuccess`
  (params (InSensor :type "HololensCameraSensor Object Reference"))
  ;[1 1 1] Setup Sensor Objects
  (`self.SetupPublishDepthImageMessageListener` (stale `CreateSensorObject` _output_get_2)))

(event `SetupPublishVLCImageMessageListener`
  (params (VLCCameraObject :type "HololensVLCCam Object Reference"))
  ;[1 1 1] Image Publisher
  (add `self.PublishMonoCamera` (delegate `OnVLCCaptureHeard`)))

(event `SetupPublishDepthImageMessageListener`
  (params (DepthCameraObject :type "HololensDepthCam Object Reference"))
  ;[1 1 1] Depth Publisher
  (add `self.PublishMonoCamera` (delegate `OnDepthCaptureHeard`)))

(event `OnVLCCaptureHeard` :!signature `self.PublishMonoCamera`
  (params (PublishPeriod :type "Float (double-precision)") (PublishData :type Boolean) (Namespace :type String))
  ;[1 1 1] Image Publisher
  (`KismetSystemLibrary.K2_SetTimerDelegate` (delegate `OnImagePubLoopTrigger`) (`self.PublishPeriod`) PublishData))

(event `OnDepthCaptureHeard` :!signature `self.PublishMonoCamera`
  (params (PublishPeriod :type "Float (double-precision)") (PublishData :type Boolean) (Namespace :type String))
  ;[1 1 1] Depth Publisher
  (`KismetSystemLibrary.K2_SetTimerDelegate` (delegate `OnDepthPubLoopTrigger`) (`self.PublishPeriod`) PublishData))

(event `OnImagePubLoopTrigger`
  ;[1 1 1] Image Publisher
  (if (stale `OnVLCCaptureHeard` PublishData)
    (bind (_outdata _outheight _outwidth _returnvalue) (`HololensVLCCam.GetVlcCamData` (stale `SetupPublishVLCImageMessageListener` VLCCameraObject)))
    (if _returnvalue
      (`RobofleetBPFunctionLibrary.PublishVLCImageMsg` (`self.ImageTopicName`) (`self.Namespace`) (make `ImageROS` (struct :`stamp` (struct)) _outheight _outwidth "mono8" 0 _outwidth _outdata))
      (else
        (`KismetSystemLibrary.PrintString` "Get VLC Cam Data Capture Failed")))
    (else
      (`RobofleetBPFunctionLibrary.PublishEmptyMsg` (`KismetStringLibrary.Concat_StrStr` (`self.PrefixTopicName`) "/stop") (`self.Namespace`)))))

(event `OnDepthPubLoopTrigger`
  ;[1 1 1] Depth Publisher
  (if (stale `OnDepthCaptureHeard` PublishData)
    (bind (_outdata _outheight _outwidth _returnvalue) (`HololensDepthCam.GetDepthCamShortThrowData` (stale `SetupPublishDepthImageMessageListener` DepthCameraObject)))
    (if _returnvalue
      (`RobofleetBPFunctionLibrary.PublishVLCImageMsg` (`self.ImageTopicName`) (`self.Namespace`) (make `ImageROS` (struct :`stamp` (struct)) _outheight _outwidth "mono8" 0 _outwidth _outdata))
      (else
        (`KismetSystemLibrary.PrintString` "Get  Depth Data Failed")))
    (else
      (`RobofleetBPFunctionLibrary.PublishEmptyMsg` (`KismetStringLibrary.Concat_StrStr` (`self.PrefixTopicName`) "/stop") (`self.Namespace`)))))

(fn `UserConstructionScript`)