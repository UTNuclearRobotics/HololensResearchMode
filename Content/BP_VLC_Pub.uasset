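; Publishes grayscale frames from a selected HoloLens visible light camera (VLC) as ROS-style raw image messages.
; BeginPlay builds topic names from the sensor type and starts capture, whose texture-created callback creates a dynamic material and starts a looping publish timer.
; Each tick, if publishing is enabled, sends the camera data as mono8; the compressed topic name is never published to.
; An aspect-scaled in-scene preview plane exists but is never triggered here.
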(event `self.ReceiveBeginPlay`
  ;[1 1 1] Event Begin Play: Setup camera and listen for data
  (`self.SetupTopicName`)
  (bind _returnvalue (`HololensResearchModeFunctionLibrary.CreateSensor` (`self.SensorType`) self))
  (bind _ashololens_vlccam (cast `HololensVLCCam` _returnvalue)
    (:`then`
      (bind _output_get (set `self.Hololens Sensor Cam` _ashololens_vlccam))
      (add `HololensCameraSensor.OnVideoTextureCreated` _output_get (delegate `OnSensorCamCreated`))
      (`HololensSensor.StartCapturing` _output_get))
    (:`CastFailed`
      (`KismetSystemLibrary.PrintString` "Cast Failed"))))

(event `OnSensorCamCreated`
  (params (InSensor :type "HololensCameraSensor Object Reference"))
  ;[1 1 1] Event Begin Play: Setup camera and listen for data
  (bind _returnvalue (`KismetMaterialLibrary.CreateDynamicMaterialInstance` "/HololensResearchMode/Materials/ResearchCamTextureMaterial.ResearchCamTextureMaterial" "None" "Transient"))
  (set `self.DynamicMaterial` _returnvalue)
  (`self.PublishRawImageMessage` (`self.PublishFrequency`)))

(event `VisualizeCameraStreamInScene`
  (bind _dynamicmaterial (`self.DynamicMaterial`))
  (bind _imageplane (`self.ImagePlane`))
  ;[1 1 1] Stream the camera feed to users view in scene
  (`SceneComponent.SetHiddenInGame` _imageplane false false)
  (`SceneComponent.SetVisibility` _imageplane true false)
  (`MaterialInstanceDynamic.SetTextureParameterValue` _dynamicmaterial "Param" (`HololensCameraSensor.CameraImage` (`self.Hololens Sensor Cam`)))
  (`PrimitiveComponent.SetMaterial` (`self.ImagePlane`) 0 _dynamicmaterial)
  (bind (_outsensorwidth _outsensorheight) (`HololensCameraSensor.GetHololensSensorResolution` (`self.Hololens Sensor Cam`)))
  (bind _output_get (set `self.Out Sensor Width` _outsensorwidth))
  (bind _output_get_2 (set `self.Out Sensor Height` _outsensorheight))
  (bind _scale (`self.CalculateImageScale` _output_get _output_get_2))
  (`SceneComponent.SetRelativeScale3D` (`self.ImagePlane`) _scale))

(event `PublishRawImageMessage`
  (params (Time :type "Float (single-precision)"))
  ;[1 1 1] Publish RAW image data
  (`KismetSystemLibrary.K2_SetTimerDelegate` (delegate `OnPubLoopTrigger`) Time true))

(event `SetupTopicName`
  (bind _returnvalue (`KismetStringLibrary.Replace` (`|GetEnumeratorNameAsString` (`self.SensorType`)) " "))
  ;[1 1 1] Setup camera topic name
  (bind _output_get (set `self.ImageTopicName` (`KismetStringLibrary.Concat_StrStr` _returnvalue "/image/raw")))
  (bind _output_get_2 (set `self.ComrpessedImageTopicName` (`KismetStringLibrary.Concat_StrStr` _returnvalue "/image/compressed")))
  (`KismetSystemLibrary.PrintString` (`KismetStringLibrary.Concat_StrStr` "Raw Image Topic Name: " _output_get "; Compressed Image Topic Name: " _output_get_2)))

(event `OnPubLoopTrigger`
  ;[1 1 1] Publish RAW image data
  (if (`self.PublishImageMessage`)
    (bind (_outdata _outheight _outwidth _returnvalue) (`HololensVLCCam.GetVlcCamData` (`self.Hololens Sensor Cam`)))
    (if _returnvalue
      (`RobofleetBPFunctionLibrary.PublishVLCImageMsg` (`self.ImageTopicName`) (`self.Namespace`) (make `ImageROS` (struct :`stamp` (struct)) _outheight _outwidth "mono8" 0 _outwidth _outdata))
      (else
        (`KismetSystemLibrary.PrintString` "Get VLC Cam Data Capture Failed")))))

(fn `CalculateImageScale`
  (params (ImageWidth :type Integer) (ImageHeight :type Integer))
  (returns (Scale :type "Vector Structure"))
  (bind _returnvalue (/ (`KismetMathLibrary.Conv_IntToDouble` ImageWidth) (`KismetMathLibrary.Conv_IntToDouble` ImageHeight)))
  (return (`KismetMathLibrary.MakeVector` (`KismetMathLibrary.FMax` _returnvalue 1.0) 1.0 (`KismetMathLibrary.FMax` (/ 1.0 _returnvalue) 1.0))))

(fn `UserConstructionScript`)