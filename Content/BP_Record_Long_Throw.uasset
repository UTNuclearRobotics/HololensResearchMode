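; BP_Record_Long_Throw toggles image message publishing for a HoloLens sensor, by its name the long-throw depth sensor, to record during gesture capture.
; On BeginPlay it binds handlers to the MRPawnMain start and stop gesture capture events, with stop noted as a voice command.
; The handlers set the PublishImageMessage flag, and stopping also publishes an empty message on a "/stop" topic derived from SensorType in the hololens namespace.
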(event `self.ReceiveBeginPlay`
  (`parent.ReceiveBeginPlay`)
  (`self.SetupStartCapture`)
  (`self.SetupStopCapture`))

(event `SetupStartCapture`
  (bind _asmrpawn_main (cast `/Game/Representations/MRPawnMain` (`GameplayStatics.GetPlayerPawn` 0)))
  (add `/Game/Representations/MRPawnMain.StartGestureCapture` _asmrpawn_main (delegate `OnStartGestureCaptureCommand`)))

(event `OnStartGestureCaptureCommand`
  (set `self.PublishImageMessage` true)
  (`KismetSystemLibrary.PrintString` "Started Publishing Message"))

(event `SetupStopCapture`
  (bind _asmrpawn_main (cast `/Game/Representations/MRPawnMain` (`GameplayStatics.GetPlayerPawn` 0)))
  ;[1 1 1] Voice Command: "Stop Gesture Capture"
  (add `/Game/Representations/MRPawnMain.StopGestureCapture` _asmrpawn_main (delegate `OnStopGestureCaptureCommand`)))

(event `OnStopGestureCaptureCommand`
  (set `self.PublishImageMessage` false)
  (`RobofleetBPFunctionLibrary.PublishEmptyMsg` (`KismetStringLibrary.Concat_StrStr` (`KismetStringLibrary.Replace` (`|GetEnumeratorNameAsString` (`self.Sensor Type`)) " ") "/stop") "hololens")
  (`KismetSystemLibrary.PrintString` "Stopped Publishing Message"))

(fn `UserConstructionScript`
  (`parent.UserConstructionScript`))