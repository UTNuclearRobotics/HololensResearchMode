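; HoloLens IMU publisher that sends sensor data as a ROS-style Imu message on the hololens namespace's imu topic.
; BeginPlay starts accelerometer and gyroscope capture and binds a publish event; magnetometer setup exists but is never called.
; Each event combines the supplied orientation with the latest sensor frames, converted to right-handed radians and meters.
; A helper extracts orientation covariance entries by index but is not called here.
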(event `self.ReceiveBeginPlay`
  ;[1 1 1] Event Begin Play
  (`self.Accelerometer`)
  (`self.Gyroscope`)
  (`self.SetupPublishImuData`))

(event `Gyroscope`
  ;[1 1 1] Gyroscope
  (bind _returnvalue (`HololensResearchModeFunctionLibrary.CreateSensor` "IMU_GYRO" self))
  (bind _ashololens_gyroscope (cast `HololensGyroscope` _returnvalue))
  (bind _output_get (set `self.As Hololens Gyroscope` _ashololens_gyroscope))
  (`HololensSensor.StartCapturing` _output_get)
  (`KismetSystemLibrary.PrintString` "Started Capturing Gyro data"))

(event `Accelerometer`
  ;[1 1 1] Accelerometer
  (bind _returnvalue (`HololensResearchModeFunctionLibrary.CreateSensor` "IMU_ACCEL" self))
  (bind _ashololens_accelerometer (cast `HololensAccelerometer` _returnvalue))
  (bind _output_get (set `self.As Hololens Accelerometer` _ashololens_accelerometer))
  (`HololensSensor.StartCapturing` _output_get)
  (`KismetSystemLibrary.PrintString` "Started Capturing IMU data"))

(event `Magnetometer`
  ;[1 1 1] Magnetometer
  (bind _returnvalue (`HololensResearchModeFunctionLibrary.CreateSensor` "IMU_MAG" self))
  (bind _ashololens_magnetometer (cast `HololensMagnetometer` _returnvalue))
  (bind _output_get (set `self.As Hololens Magnetometer` _ashololens_magnetometer))
  (`HololensSensor.StartCapturing` _output_get)
  (`KismetSystemLibrary.PrintString` "started Capturing Imu data"))

(event `SetupPublishImuData`
  ;[1 1 1] Publish Data
  (add `self.PublishImuMessage` (delegate `OnPublishImuMsgHeard`)))

(event `OnPublishImuMsgHeard` :!signature `self.PublishImuMessage`
  (params (ImuMsgOrientation :type "Rotator Structure") (ImuMsgCovariance :type "Array of Float (double-precision) (by ref)"))
  (bind _estimatedcovariance (`self.EstimatedCovariance`))
  ;[1 1 1] Publish Data
  (bind _frame (`HololensGyroscope.GetGyroscopeFrame` (`self.As Hololens Gyroscope`))) ; Angular Velocity (deg/s)
  (bind _returnvalue (`RobofleetBPFunctionLibrary.ConvertDegToRad` (`.GyroSample` (break `HololensGyroscopeFrame` _frame)))) ; Convert to (rad/s)
  (bind _returnvalue_2 (`RobofleetBPFunctionLibrary.ConvertAngleToRightHand` _returnvalue)) ; Convert to right hand coords
  (bind _frame_2 (`HololensAccelerometer.GetAccelerometerFrame` (`self.As Hololens Accelerometer`))) ; Linear Acceleration (cm/s^2)
  (bind _returnvalue_3 (`RobofleetBPFunctionLibrary.ConvertPositionToRightHandMeters` (`.AccelSample` (break `HololensAccelerometerFrame` _frame_2)))) ; Convert to m/s^2
  (bind _output_get (set `self.ImuMsg` (make `Imu` (make `Header` 0 (struct) "camera_imu_optical_frame") (`self.Imu Msg Orientation`) (`self.Imu Msg Orientation Covariance`) _returnvalue_2 _estimatedcovariance _returnvalue_3 _estimatedcovariance)))
  (`RobofleetBPFunctionLibrary.PublishImuMsg` "imu" "hololens" _output_get))

(fn `GetOrientationValues`
  (params (CovarianceMatrix :type "Array of Float (double-precision)"))
  (returns (OrientationCovarianceMatrix :type "Array of Float (double-precision)"))
  (locals (OrientationIndices :type "Array of Integer") (OrientationCovariance :type "Array of Float (double-precision)"))
  (for (_array_element _array_index) CovarianceMatrix
    (for _array_element_2 (`local.OrientationIndices`)
      (if (== _array_index _array_element_2)
        (`KismetArrayLibrary.Array_Add` (`local.OrientationCovariance`) _array_element))))
  (return (`local.OrientationCovariance`)))

(fn `UserConstructionScript`)