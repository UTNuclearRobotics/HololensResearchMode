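; Blueprint that starts and stops hand gesture recording on HoloLens through voice commands.
; After staggered delays on BeginPlay, it binds handlers to the MRPawnMain start and stop gesture capture commands.
; The handlers toggle the PublishImageMessage flag to control sensor image publishing.
; Stopping also publishes an empty message on a "/stop" topic built from the sensor type name, under the hololens namespace.
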(event `self.ReceiveBeginPlay`
  (`parent.ReceiveBeginPlay`)
  (`KismetSystemLibrary.Delay` 5.0)
  (`self.SetupStartCapturingGesture`)
  (`KismetSystemLibrary.Delay` 10.0)
  (`self.SetupStopCapturingGesture`))

(event `SetupStartCapturingGesture`
  (bind _asmrpawn_main (cast `/Game/Representations/MRPawnMain` (`GameplayStatics.GetPlayerPawn` 0)))
  ;[1 1 1] Voice Command: "Start Gesture Capture"
  (add `/Game/Representations/MRPawnMain.StartGestureCapture` _asmrpawn_main (delegate `OnStartGestureCaptureCommand`)))

(event `OnStartGestureCaptureCommand`
  (set `self.PublishImageMessage` true)
  (`KismetSystemLibrary.PrintString` "Started Publishing Message"))

(event `SetupStopCapturingGesture`
  (bind _asmrpawn_main (cast `/Game/Representations/MRPawnMain` (`GameplayStatics.GetPlayerPawn` 0)))
  ;[1 1 1] Voice Command: "Stop Gesture Capture"
  (add `/Game/Representations/MRPawnMain.StopGestureCapture` _asmrpawn_main (delegate `OnStopGestureCaptureCommand`)))

(event `OnStopGestureCaptureCommand`
  (set `self.PublishImageMessage` false)
  (`RobofleetBPFunctionLibrary.PublishEmptyMsg` (`KismetStringLibrary.Concat_StrStr` (`KismetStringLibrary.Replace` (`|GetEnumeratorNameAsString` (`self.SensorType`)) " ") "/stop") "hololens")
  (`KismetSystemLibrary.PrintString` "Stopped Publishing Message"))

(fn `UserConstructionScript`
  (`parent.UserConstructionScript`))