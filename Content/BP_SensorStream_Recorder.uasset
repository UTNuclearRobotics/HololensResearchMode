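; Sensor stream recorder that spawns capture actors for four mono cameras to record hand gestures.
; After a startup delay, BeginPlay spawns one BP_Record_Hand_Gesture per camera, passing the publish period and capture word.
; An optional DepthPub event spawns a short- or long-throw depth recorder by sensor type, but its call is left disconnected.
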(event `self.ReceiveBeginPlay`
  (`KismetSystemLibrary.Delay` 15.0)
  (`self.VlcPub`) ; Event to start publishing the 4 Mono Cameras
)

(event `VlcPub`
  (bind _publishperiod (`self.PublishPeriod`))
  (bind _captureword (`self.CaptureWord`))
  (`|SpawnActorFromClass` "/HololensResearchMode/BP_Record_Hand_Gesture.BP_Record_Hand_Gesture_C" (`KismetMathLibrary.MakeTransform` (0.0 0.0 0.0)) "Undefined" "OverrideRootScale" null "LEFT_LEFT" _publishperiod false _captureword null)
  (`|SpawnActorFromClass` "/HololensResearchMode/BP_Record_Hand_Gesture.BP_Record_Hand_Gesture_C" (`KismetMathLibrary.MakeTransform` (0.0 0.0 0.0)) "Undefined" "OverrideRootScale" null "LEFT_FRONT" _publishperiod false _captureword null)
  (`|SpawnActorFromClass` "/HololensResearchMode/BP_Record_Hand_Gesture.BP_Record_Hand_Gesture_C" (`KismetMathLibrary.MakeTransform` (0.0 0.0 0.0)) "Undefined" "OverrideRootScale" null "RIGHT_FRONT" _publishperiod false _captureword null)
  (`|SpawnActorFromClass` "/HololensResearchMode/BP_Record_Hand_Gesture.BP_Record_Hand_Gesture_C" (`KismetMathLibrary.MakeTransform` (0.0 0.0 0.0)) "Undefined" "OverrideRootScale" null "RIGHT_RIGHT" _publishperiod false _captureword null)
  (`KismetSystemLibrary.PrintString` "Spawned Gesture Capture"))

(event `DepthPub`
  (params (DepthSensorType :type "EHololensSensorType Enum" :default "LEFT_FRONT"))
  (switch `EHololensSensorType` DepthSensorType
    (:`DEPTH_AHAT`
      (`|SpawnActorFromClass` "/HololensResearchMode/BP_Record_Short_Throw.BP_Record_Short_Throw_C" (`KismetMathLibrary.MakeTransform` (0.0 0.0 0.0)) "Undefined" "OverrideRootScale" null "DEPTH_AHAT" (`self.PublishPeriod`) "hololens" null))
    (:`DEPTH_LONG_THROW`
      (`|SpawnActorFromClass` "/HololensResearchMode/BP_Record_Long_Throw.BP_Record_Long_Throw_C" (`KismetMathLibrary.MakeTransform` (0.0 0.0 0.0)) "Undefined" "OverrideRootScale" null "DEPTH_LONG_THROW" (`self.PublishPeriod`) "hololens" null))))

(fn `UserConstructionScript`)